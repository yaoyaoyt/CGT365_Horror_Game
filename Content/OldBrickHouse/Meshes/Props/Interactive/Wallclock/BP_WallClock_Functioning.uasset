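; Animated wall clock prop with a swinging pendulum and stepping hands, running faster than real time.
; A timeline started on BeginPlay lerps the pendulum's rotation between two angles and ping-pongs by reversing each time it finishes.
; Tick drives chained Delay nodes that act as repeating timers, stepping the minute hand every few seconds and the hour hand roughly once per minute-hand revolution, independent of any clock time.
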(event `self.ReceiveBeginPlay`
  (bind (_direction _pendulum_movement) (`Timeline|Timeline` :!label _label)
    (:`Update`
      (`SceneComponent.K2_SetRelativeRotation` (`self.SM_Wallclock_Pendulum`) (`KismetMathLibrary.RLerp` (struct :`Roll` 20.0) (struct :`Roll` -20.0) _pendulum_movement) false false))
    (:`Finished`
      (if (== _direction 0)
        (goto _label :!via `Reverse`)
        (else
          (goto _label))))))

(event `self.ReceiveTick`
  (params (DeltaSeconds :type "Float (single-precision)"))
  (bind _sm_minute_hand (`self.SM_Minute_Hand`))
  (bind _sm_hour_hand (`self.SM_Hour_Hand`))
  (bind (_relativerotation_roll _relativerotation_pitch _relativerotation_yaw) (`KismetMathLibrary.BreakRotator` (`SceneComponent.RelativeRotation` _sm_hour_hand)))
  (bind (_relativerotation_roll_2 _relativerotation_pitch_2) (`KismetMathLibrary.BreakRotator` (`SceneComponent.RelativeRotation` _sm_minute_hand)))
  (`KismetSystemLibrary.Delay` 5.0)
  (`SceneComponent.K2_SetRelativeRotation` _sm_minute_hand (`KismetMathLibrary.MakeRotator` (+ _relativerotation_roll_2 -6.0) _relativerotation_pitch_2) false false)
  (`KismetSystemLibrary.Delay` 301.0)
  (`SceneComponent.K2_SetRelativeRotation` _sm_hour_hand (`KismetMathLibrary.MakeRotator` (+ _relativerotation_roll -30.0) _relativerotation_pitch _relativerotation_yaw) false false))

(fn `UserConstructionScript`)