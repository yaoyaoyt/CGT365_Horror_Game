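; Broken wall clock prop that the player can interact with in the game.
; Overlap shows an Interact widget and enables input, and pressing E snaps the actor to a fixed rotation and destroys its Box component.
; Ping-pong timelines swing the pendulum and twitch the minute hand between two angles.
; Tick uses chained Delays to step the minute and hour hands, with both it and the timeline writing the minute hand's rotation.
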(event `self.ReceiveActorBeginOverlap`
  (params (OtherActor :type "Actor Object Reference"))
  ;[1 1 1] Interact Prompt
  (bind _returnvalue (`|CreateWidget` "/Game/CGT365Stuff/interact.interact_C"))
  (`UserWidget.AddToViewport` _returnvalue 0)
  ;[1 1 1] Allows for interaction
  (`self.EnableInput` (`GameplayStatics.GetPlayerController` 0)))

(event `self.ReceiveActorEndOverlap`
  (params (OtherActor :type "Actor Object Reference"))
  ;[1 1 1] Interact Prompt
  (`Widget.RemoveFromParent` (stale `self.ReceiveActorBeginOverlap` _returnvalue))
  ;[1 1 1] Allows for interaction
  (`self.DisableInput` (`GameplayStatics.GetPlayerController` 0)))

(event `Key|E`
  (params (Key :type "Key Structure"))
  (:`Pressed`
    (bind _asbp_wall_clock_broken (cast `/Game/OldBrickHouse/Meshes/Props/Interactive/Wallclock/BP_WallClock_Broken` self))
    (`self.K2_SetActorRotation` _asbp_wall_clock_broken (struct :`Yaw` 180.0) false)
    (`ActorComponent.K2_DestroyComponent` (`self.Box`))))

(event `self.ReceiveBeginPlay`
  (bind (_direction _pendulum_movement) (`Timeline|Timeline` :!label _label)
    (:`Update`
      (`SceneComponent.K2_SetRelativeRotation` (`self.SM_Wallclock_Pendulum`) (`KismetMathLibrary.RLerp` (struct :`Roll` -20.0) (struct :`Roll` 5.0) _pendulum_movement) false false)
      (bind (_direction_2 _minute_hand) (`Timeline|Minute Hand` :!label _label_2)
        (:`Update`
          (`SceneComponent.K2_SetRelativeRotation` (`self.SM_Minute_Hand`) (`KismetMathLibrary.RLerp` (struct :`Roll` -168.0) (struct :`Roll` -180.0) _minute_hand) false false))
        (:`Finished`
          (if (== _direction_2 0)
            (goto _label_2 :!via `Reverse`)
            (else
              (goto _label_2))))))
    (:`Finished`
      (if (== _direction 0)
        (goto _label :!via `Reverse`)
        (else
          (goto _label))))))

(event `self.ReceiveTick`
  (params (DeltaSeconds :type "Float (single-precision)"))
  (bind _sm_minute_hand (`self.SM_Minute_Hand`))
  (bind _sm_hour_hand (`self.SM_Hour_Hand`))
  (bind (_relativerotation_roll _relativerotation_pitch _relativerotation_yaw) (`KismetMathLibrary.BreakRotator` (`SceneComponent.RelativeRotation` _sm_hour_hand)))
  (bind (_relativerotation_roll_2 _relativerotation_pitch_2) (`KismetMathLibrary.BreakRotator` (`SceneComponent.RelativeRotation` _sm_minute_hand)))
  (`KismetSystemLibrary.Delay` 5.0)
  (`SceneComponent.K2_SetRelativeRotation` _sm_minute_hand (`KismetMathLibrary.MakeRotator` (+ _relativerotation_roll_2 -6.0) _relativerotation_pitch_2) false false)
  (`KismetSystemLibrary.Delay` 301.0)
  (`SceneComponent.K2_SetRelativeRotation` _sm_hour_hand (`KismetMathLibrary.MakeRotator` (+ _relativerotation_roll -30.0) _relativerotation_pitch _relativerotation_yaw) false false))

(fn `UserConstructionScript`)