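; BP_DialogueManager is a level actor that wires up the dialogue system when play begins.
; It creates a single UI_DialogueDisplay widget, then finds every BP_DialogueController and Interactable_parent actor in the world.
; Each found actor receives the shared widget and a reference back to the manager, so all dialogue sources use one display.
; The manager has no other runtime logic.
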(event `self.ReceiveBeginPlay`
  (bind _returnvalue (`|GenericCreateObject` "/Game/CGT365Stuff/BP_Dialogue/UI_DialogueDisplay.UI_DialogueDisplay_C"))
  (`|ExecutionSequence`
    (:`then_0`
      (bind _outactors (`GameplayStatics.GetAllActorsOfClass` "/Game/CGT365Stuff/BP_Dialogue/BP_DialogueController.BP_DialogueController_C"))
      (for _array_element _outactors
        (`/Game/CGT365Stuff/BP_Dialogue/BP_DialogueController.Set UIBP` _array_element _returnvalue)
        (`/Game/CGT365Stuff/BP_Dialogue/BP_DialogueController.Set Manager Ref` _array_element self)))
    (:`then_1`
      (bind _outactors_2 (`GameplayStatics.GetAllActorsOfClass` "/Game/CGT365Stuff/Interactables/Interactable_parent.Interactable_parent_C"))
      (for _array_element_2 _outactors_2
        (`/Game/CGT365Stuff/Interactables/Interactable_parent.Set UIBP` _array_element_2 _returnvalue)
        (`/Game/CGT365Stuff/Interactables/Interactable_parent.Set Manager Ref` _array_element_2 self)))))

(fn `UserConstructionScript`)