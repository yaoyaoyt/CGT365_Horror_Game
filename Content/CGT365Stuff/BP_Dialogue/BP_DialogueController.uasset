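; Proximity trigger actor that shows dialogue description and interaction prompt text when the first-person character enters its radius-sized sphere.
; Conditional triggers first count matches between their required conditions and the manager's unlocked conditions.
; An injected UI widget displays single descriptions or queued sequences, and hides them on exit.
; Non-repeatable triggers destroy themselves on the next qualifying overlap after displaying.
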(event `self.ReceiveBeginPlay`
  (`SphereComponent.SetSphereRadius` (`self.Sphere`) (`self.Radius`) true))

(event `self.Sphere.OnComponentBeginOverlap`
  (params (OverlappedComponent :type "PrimitiveComponent Object Reference") (OtherActor :type "Actor Object Reference") (OtherComp :type "PrimitiveComponent Object Reference") (OtherBodyIndex :type Integer) (bFromSweep :type Boolean) (SweepResult :type "HitResult Structure (by ref)"))
  (bind _widget_bp (`self.Widget BP`))
  (cast `/Game/FirstPerson/Blueprints/BP_FirstPersonCharacter` OtherActor)
  (if (`self.Is conditional`)
    (bind _conditons_met (`self.Check if conditions are met` (`self.Conditions`) (`/Game/CGT365Stuff/BP_Dialogue/BP_DialogueManager.UnlockedCondition` (`self.Manager Ref`))))
    (if _conditons_met
      (if (`self.IsRepeated`) :!label _label
        (if (`self.Repeatable`)
          (`|ExecutionSequence` :!label _label_2
            (:`then_0`
              (if (`self.DoShowInteraction`)
                (`/Game/CGT365Stuff/BP_Dialogue/UI_DialogueDisplay.Display Interaction` _widget_bp (`self.Interaction Text`))))
            (:`then_1`
              (if (`self.DoShowDescription`)
                (if (`self.IsSequence`)
                  (`/Game/CGT365Stuff/BP_Dialogue/UI_DialogueDisplay.Push List To Display` _widget_bp (`self.Description Sequence`))
                  (else
                    (`/Game/CGT365Stuff/BP_Dialogue/UI_DialogueDisplay.Display Description` _widget_bp (`self.Description Text`))))))
            (:`then_2`
              (`UserWidget.AddToViewport` (`self.Widget BP`) 0)
              (set `self.IsRepeated` true)))
          (else
            (`self.K2_DestroyActor`)))
        (else
          (goto _label_2))))
    (else
      (goto _label))))

(event `self.Sphere.OnComponentEndOverlap`
  (params (OverlappedComponent :type "PrimitiveComponent Object Reference") (OtherActor :type "Actor Object Reference") (OtherComp :type "PrimitiveComponent Object Reference") (OtherBodyIndex :type Integer))
  (bind _widget_bp (`self.Widget BP`))
  (cast `/Game/FirstPerson/Blueprints/BP_FirstPersonCharacter` OtherActor)
  (`|ExecutionSequence`
    (:`then_0`
      (if (`self.DoShowDescription`)
        (`/Game/CGT365Stuff/BP_Dialogue/UI_DialogueDisplay.Set Invisible Description` _widget_bp)))
    (:`then_1`
      (if (`self.DoShowInteraction`)
        (`/Game/CGT365Stuff/BP_Dialogue/UI_DialogueDisplay.Set Invisible Interaction` _widget_bp)))))

(fn `Check if conditions are met`
  (params (`Required Condition` :type "Array of String") (`Met Conditions` :type "Array of String"))
  (returns (`Conditons Met` :type Boolean))
  (locals (Unmet :type Boolean) (`match count` :type Integer))
  (for _array_element `Required Condition`
    (for _array_element_2 `Met Conditions`
      (if (`KismetStringLibrary.EqualEqual_StrStr` _array_element _array_element_2)
        (`/Engine/EditorBlueprintResources/StandardMacros.IncrementInt` (`local.match count`)))))
  (return (== (`KismetArrayLibrary.Array_Length` `Required Condition`) (`local.match count`))))

(fn `Set Manager Ref`
  (params (Ref :type "/Game/CGT365Stuff/BP_Dialogue/BP_DialogueManager Object Reference"))
  (set `self.Manager Ref` Ref))

(fn `Set UIBP`
  (params (Reference :type "/Game/CGT365Stuff/BP_Dialogue/UI_DialogueDisplay Object Reference"))
  (set `self.Widget BP` Reference))

(fn `UserConstructionScript`)